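; Point light actor that flickers and jitters around its spawn location, with exposed-style variables for intensity, color and radius applied in the construction script.
; Each Tick blends the previous intensity toward a randomized value around the base intensity.
; It also eases the actor toward random offsets from the location stored at BeginPlay.
; Smoothing is a per-frame Lerp independent of delta time, so flicker speed follows frame rate.
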(event EventBeginPlay
  (bind _returnvalue (Transformation|GetActorLocation))
  (Variables|Default|SetStartLocation _returnvalue)
  (Variables|Default|SetOldLocation _returnvalue))

(event EventTick
  (params (DeltaSeconds :type Float%20%28single-precision%29))
  (Rendering|Components|Light|SetIntensity (Variables|Default|GetPointLight1) (Math|Float|Lerp (Variables|Default|GetOld_Intensity) (+ (Variables|Default|GetLight%20Intensity) (Math|Random|RandomFloatinRange -1e+03 1e+03)) 0.6))
  (Variables|Default|SetOld_Intensity (Math|Float|Lerp (Variables|Default|GetOld_Intensity) (+ (Variables|Default|GetLight%20Intensity) (Math|Random|RandomFloatinRange -1e+03 1e+03)) 0.6))
  (Transformation|SetActorLocation (Math|Vector|Lerp(Vector) (+ (Variables|Default|GetStartLocation) (* (Math|Random|RandomUnitVector) (Math|Random|RandomFloatinRange -4e+01 4e+01))) (Variables|Default|GetOldLocation) 0.9) false)
  (Variables|Default|SetOldLocation (Math|Vector|Lerp(Vector) (+ (Variables|Default|GetStartLocation) (* (Math|Random|RandomUnitVector) (Math|Random|RandomFloatinRange -4e+01 4e+01))) (Variables|Default|GetOldLocation) 0.9)))

(fn ConstructionScript
  (bind _pointlight1 (Variables|Default|GetPointLight1))
  (Rendering|Components|Light|SetIntensity _pointlight1 (Variables|Default|GetLight%20Intensity))
  (Rendering|Components|Light|SetLightColor _pointlight1 (Variables|Default|GetLight%20Color))
  (Rendering|Lighting|SetAttenuationRadius _pointlight1 (Variables|Default|GetLight_Radius)))