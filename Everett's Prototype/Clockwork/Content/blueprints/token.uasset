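; Grid token actor that steps one cell at a time across Basic_Cell actors in response to four directional move events.
; BeginPlay caches all cells and snaps the token to the 100-unit grid.
; Move finds cells by linear search, stepping only if the current exit is open and the neighbor has Tracks and a matching open side.
; Tick lerps location toward the grid coordinates and rotation toward CurrentAngle, which stays zero here.
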(event Custom|move_right
  ;[1 1 1] Move
  (CallFunction|Move 1 1))

(event Custom|move_down
  ;[1 1 1] Move
  (CallFunction|Move 2 0 1))

(event Custom|move_left
  ;[1 1 1] Move
  (CallFunction|Move 3 -1))

(event Custom|move_up
  ;[1 1 1] Move
  (CallFunction|Move 0 0 -1))

(event EventBeginPlay
  (bind _returnvalue (Transformation|GetActorLocation))
  (bind (_x _y) (Math|Vector|BreakVector _returnvalue))
  ;[1 1 1] Startup
  (bind _outactors (Actor|GetAllActorsOfClass "/Game/blueprints/Cells/Basic_Cell.Basic_Cell_C"))
  (Variables|Default|SetAll_Cells _outactors)
  (Variables|Default|SettokenX (Math|Float|Floor (/ _x 1e+02)))
  (Variables|Default|SettokenY (Math|Float|Floor (/ _y 1e+02)))
  (Transformation|SetActorLocation (Math|Vector|MakeVector (* (Math|Conversions|ToFloat(Integer) (Variables|Default|GettokenX)) 1e+02) (* (Math|Conversions|ToFloat(Integer) (Variables|Default|GettokenY)) 1e+02) 0.0) false)
  (Variables|Default|Setcurrent_angle "0, 0, 0"))

(event EventTick
  (params (DeltaSeconds :type Float%20%28single-precision%29))
  ;[1 1 1] Tick
  (Transformation|SetActorLocation (Math|Vector|Lerp(Vector) (Transformation|GetActorLocation) (Math|Vector|MakeVector (* (Math|Conversions|ToFloat(Integer) (Variables|Default|GettokenX)) 1e+02) (* (Math|Conversions|ToFloat(Integer) (Variables|Default|GettokenY)) 1e+02) 0.0) 0.3) false)
  (Transformation|SetActorRotation (Math|Rotator|Lerp(Rotator) (Transformation|GetActorRotation) (Variables|Default|Getcurrent_angle) 0.5 true)))

(fn ConstructionScript)

(fn FindCell
  (params (offsetX :type Integer) (offsetY :type Integer))
  (for (_array_element _array_index) (Variables|Default|GetAll_Cells)
    (bind _asbasic_cell (Utilities|Casting|CastToBasic_Cell _array_element))
    (Math|Integer|CompareInt (Variables|/Game/blueprints/Cells/Basic_Cell.Basic_Cell_C|GetcellX _asbasic_cell) (+ (Variables|Default|GettokenX) offsetX)
      (:==
        (Math|Integer|CompareInt (Variables|/Game/blueprints/Cells/Basic_Cell.Basic_Cell_C|GetcellY _asbasic_cell) (+ offsetY (Variables|Default|GettokenY))
          (:==
            (return _array_element _array_index)))))))

(fn Move
  (params (direction :type Integer) (offsetX :type Integer) (offsetY :type Integer))
  (bind _cell (CallFunction|FindCell))
  (bind _asbasic_cell (Utilities|Casting|CastToBasic_Cell _cell))
  (switch int direction
    (:0
      (if (Variables|/Game/blueprints/Cells/Basic_Cell.Basic_Cell_C|GetupOpen _asbasic_cell)
        (bind _cell_2 (CallFunction|FindCell offsetX offsetY :!label _label))
        (bind _asbasic_cell_2 (Utilities|Casting|CastToBasic_Cell _cell_2))
        (if (Variables|/Game/blueprints/Cells/Basic_Cell.Basic_Cell_C|Gettracks _asbasic_cell_2)
          (switch int direction
            (:0
              (if (Variables|/Game/blueprints/Cells/Basic_Cell.Basic_Cell_C|GetdownOpen _asbasic_cell_2)
                (Variables|Default|SettokenY (+ (Variables|Default|GettokenY) -1))
                (return)))
            (:1
              (if (Variables|/Game/blueprints/Cells/Basic_Cell.Basic_Cell_C|GetleftOpen _asbasic_cell_2)
                (Variables|Default|SettokenX (+ (Variables|Default|GettokenX) 1))
                (return)))
            (:2
              (if (Variables|/Game/blueprints/Cells/Basic_Cell.Basic_Cell_C|GetupOpen _asbasic_cell_2)
                (Variables|Default|SettokenY (+ (Variables|Default|GettokenY) 1))
                (return)))
            (:3
              (if (Variables|/Game/blueprints/Cells/Basic_Cell.Basic_Cell_C|GetrightOpen _asbasic_cell_2)
                (Variables|Default|SettokenX (+ (Variables|Default|GettokenX) -1))
                (return)))))))
    (:1
      (if (Variables|/Game/blueprints/Cells/Basic_Cell.Basic_Cell_C|GetrightOpen _asbasic_cell)
        (goto _label)))
    (:2
      (if (Variables|/Game/blueprints/Cells/Basic_Cell.Basic_Cell_C|GetdownOpen _asbasic_cell)
        (goto _label)))
    (:3
      (if (Variables|/Game/blueprints/Cells/Basic_Cell.Basic_Cell_C|GetleftOpen _asbasic_cell)
        (goto _label)))))