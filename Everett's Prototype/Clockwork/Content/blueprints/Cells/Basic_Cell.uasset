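; Grid cell for a track puzzle, holding an optional rotatable track piece with open/closed sides.
; Construction script sets cell and track meshes from track type and initial rotation; BeginPlay derives grid coordinates and side openings.
; Clockwise and counter-clockwise events shift the openings and target yaw, which Tick lerps toward.
; Rotating also turns the first found Token's angle when it occupies this cell.
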(event Custom|Rot_Clockwise
  ;[1 1 1] Rotation
  (CallFunction|RotateCW (Variables|Default|GetupOpen) (Variables|Default|GetrightOpen) (Variables|Default|GetdownOpen) (Variables|Default|GetleftOpen)))

(event Custom|Rot_Counter_Clockwise
  ;[1 1 1] Rotation
  (CallFunction|RotateCCW (Variables|Default|GetupOpen) (Variables|Default|GetrightOpen) (Variables|Default|GetdownOpen) (Variables|Default|GetleftOpen)))

(event EventBeginPlay
  (bind _returnvalue (Transformation|GetActorLocation))
  (bind (_x _y) (Math|Vector|BreakVector _returnvalue))
  ;[1 1 1] Startup
  (Variables|Default|SetcellX (Math|Float|Floor (/ _x 1e+02)))
  (Variables|Default|SetcellY (Math|Float|Floor (/ _y 1e+02)))
  (Variables|Default|SetwantedTrackRotation (Transformation|GetWorldRotation (Variables|Default|Gettrack_rot)))
  (switch int (Variables|Default|Gettrack_type)
    (:0
      (Variables|Default|SetupOpen true)
      (Variables|Default|SetrightOpen false)
      (Variables|Default|SetdownOpen true)
      (Variables|Default|SetleftOpen false))
    (:1
      (Variables|Default|SetupOpen true)
      (Variables|Default|SetrightOpen false)
      (Variables|Default|SetdownOpen false)
      (Variables|Default|SetleftOpen true))
    (:2
      (Variables|Default|SetupOpen true)
      (Variables|Default|SetrightOpen true)
      (Variables|Default|SetdownOpen false)
      (Variables|Default|SetleftOpen true))
    (:3
      (Variables|Default|SetupOpen true)
      (Variables|Default|SetrightOpen true)
      (Variables|Default|SetdownOpen true)
      (Variables|Default|SetleftOpen true))
    (:4
      (Variables|Default|SetupOpen true)
      (Variables|Default|SetrightOpen false)
      (Variables|Default|SetdownOpen false)
      (Variables|Default|SetleftOpen false)))
  (Utilities|FlowControl|ForLoopwithBreak 1 (Variables|Default|GetInitial_Track_Rotation)
    (:LoopBody
      (CallFunction|RotateCWStartup (Variables|Default|GetupOpen) (Variables|Default|GetrightOpen) (Variables|Default|GetleftOpen) (Variables|Default|GetdownOpen)))
    (:Completed
      (bind _outactors (Actor|GetAllActorsOfClass "/Game/blueprints/token.token_C"))
      (Variables|Default|Settoken (Utilities|Array|Get(acopy) _outactors)))))

(event EventTick
  (params (DeltaSeconds :type Float%20%28single-precision%29))
  (bind _track_rot (Variables|Default|Gettrack_rot))
  ;[1 1 1] Tick
  (Transformation|SetWorldRotation _track_rot (Math|Rotator|Lerp(Rotator) (Transformation|GetWorldRotation _track_rot) (Variables|Default|GetwantedTrackRotation) 0.5 true) false))

(fn ConstructionScript
  (bind _track (Variables|Default|Gettrack))
  (bind _track_2 (Variables|Default|Gettrack))
  (bind _track_rot (Variables|Default|Gettrack_rot))
  (bind _cell (Variables|Default|GetCell))
  (if (Variables|Default|Gettracks)
    (Components|StaticMesh|SetStaticMesh _cell (Variables|Default|Getcell_light))
    (Rendering|SetVisibility _track true false)
    (switch int (Variables|Default|Gettrack_type)
      (:0
        (Components|StaticMesh|SetStaticMesh _track_2 (Variables|Default|Getcell_track_straight)))
      (:1
        (Components|StaticMesh|SetStaticMesh _track_2 (Variables|Default|Getcell_track_corner)))
      (:2
        (Components|StaticMesh|SetStaticMesh _track_2 (Variables|Default|Getcell_track_T)))
      (:3
        (Components|StaticMesh|SetStaticMesh _track_2 (Variables|Default|Getcell_track_4way)))
      (:4
        (Components|StaticMesh|SetStaticMesh _track_2 (Variables|Default|Getcell_track_DE))))
    (switch int (Variables|Default|GetInitial_Track_Rotation)
      (:0
        (Transformation|SetWorldRotation _track_rot "0,0.000000, 0" false))
      (:1
        (Transformation|SetWorldRotation _track_rot "0,90.000000, 0" false))
      (:2
        (Transformation|SetWorldRotation _track_rot "0,180.000000, 0" false))
      (:3
        (Transformation|SetWorldRotation _track_rot "0,270.000000, 0" false)))
    (else
      (Components|StaticMesh|SetStaticMesh _cell (Variables|Default|Getcell_dark))
      (Rendering|SetVisibility _track false false))))

(fn RotateCWStartup
  (params (UpInitial :type Boolean) (RightInitial :type Boolean) (LeftInitial :type Boolean) (DownInitial :type Boolean))
  (Variables|Default|SetupOpen LeftInitial)
  (Variables|Default|SetrightOpen UpInitial)
  (Variables|Default|SetdownOpen RightInitial)
  (Variables|Default|SetleftOpen DownInitial))

(fn RotateCW
  (params (upOpen :type Boolean) (rightOpen :type Boolean) (downOpen :type Boolean) (leftOpen :type Boolean))
  (Variables|Default|SetupOpen leftOpen)
  (Variables|Default|SetrightOpen upOpen)
  (Variables|Default|SetdownOpen rightOpen)
  (Variables|Default|SetleftOpen downOpen)
  (Variables|Default|SetwantedTrackRotation (Class|KismetMathLibrary|MakeRot (.Pitch (Class|KismetMathLibrary|BreakRot (Variables|Default|GetwantedTrackRotation))) (+ (.Yaw (Class|KismetMathLibrary|BreakRot (Variables|Default|GetwantedTrackRotation))) 9e+01) (.Roll (Class|KismetMathLibrary|BreakRot (Variables|Default|GetwantedTrackRotation)))))
  (bind _astoken (Utilities|Casting|CastTotoken (Variables|Default|Gettoken)))
  (Math|Integer|CompareInt (Variables|/Game/blueprints/token.token_C|GettokenX _astoken) (Variables|Default|GetcellX)
    (:==
      (Math|Integer|CompareInt (Variables|Default|GetcellY) (Variables|/Game/blueprints/token.token_C|GettokenY _astoken)
        (:==
          (Variables|/Game/blueprints/token.token_C|Setcurrent_angle _astoken (Class|KismetMathLibrary|MakeRot (.Pitch (Class|KismetMathLibrary|BreakRot (Variables|/Game/blueprints/token.token_C|Getcurrent_angle _astoken))) (+ (.Yaw (Class|KismetMathLibrary|BreakRot (Variables|/Game/blueprints/token.token_C|Getcurrent_angle _astoken))) 9e+01) (.Roll (Class|KismetMathLibrary|BreakRot (Variables|/Game/blueprints/token.token_C|Getcurrent_angle _astoken))))))))))

(fn RotateCCW
  (params (upOpen :type Boolean) (rightOpen :type Boolean) (downOpen :type Boolean) (leftOpen :type Boolean))
  (Variables|Default|SetupOpen rightOpen)
  (Variables|Default|SetrightOpen downOpen)
  (Variables|Default|SetdownOpen leftOpen)
  (Variables|Default|SetleftOpen upOpen)
  (Variables|Default|SetwantedTrackRotation (Class|KismetMathLibrary|MakeRot (.Pitch (Class|KismetMathLibrary|BreakRot (Variables|Default|GetwantedTrackRotation))) (+ (.Yaw (Class|KismetMathLibrary|BreakRot (Variables|Default|GetwantedTrackRotation))) -9e+01) (.Roll (Class|KismetMathLibrary|BreakRot (Variables|Default|GetwantedTrackRotation)))))
  (bind _astoken (Utilities|Casting|CastTotoken (Variables|Default|Gettoken)))
  (Math|Integer|CompareInt (Variables|/Game/blueprints/token.token_C|GettokenX _astoken) (Variables|Default|GetcellX)
    (:==
      (Math|Integer|CompareInt (Variables|Default|GetcellY) (Variables|/Game/blueprints/token.token_C|GettokenY _astoken)
        (:==
          (Variables|/Game/blueprints/token.token_C|Setcurrent_angle _astoken (Class|KismetMathLibrary|MakeRot (.Pitch (Class|KismetMathLibrary|BreakRot (Variables|/Game/blueprints/token.token_C|Getcurrent_angle _astoken))) (+ (.Yaw (Class|KismetMathLibrary|BreakRot (Variables|/Game/blueprints/token.token_C|Getcurrent_angle _astoken))) -9e+01) (.Roll (Class|KismetMathLibrary|BreakRot (Variables|/Game/blueprints/token.token_C|Getcurrent_angle _astoken))))))))))