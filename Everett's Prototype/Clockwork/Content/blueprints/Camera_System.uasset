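; Camera rig Blueprint that rotates its CameraMover component from camera axis input while Cam_Move is held.
; Each Tick, inverted input is blended heavily with the previous rotation delta for smoothing, without delta-time scaling.
; On release, the stored delta decays toward zero, so the camera glides to a stop.
; Pitch is then clamped to a downward-looking range, while yaw is unrestricted.
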(event EventTick
  (params (DeltaSeconds :type Float%20%28single-precision%29))
  (bind _camera_mover (Variables|Default|GetCamera_Mover))
  (bind _relativerotation (Variables|/Script/Engine.SceneComponent|GetRelativeRotation _camera_mover))
  (bind (_pitch _yaw _roll) (Class|KismetMathLibrary|BreakRot _relativerotation))
  (if (Variables|Default|GetCam_Moving)
    (Transformation|AddRelativeRotation (Math|Rotator|Lerp(Rotator) (Class|KismetMathLibrary|MakeRot (* (Input|AxisValues|GetCam_Y) -1.0) (* (Input|AxisValues|GetCam_X) -1.0) 0.0) (Variables|Default|GetOld_Rotator) 0.9) false)
    (Variables|Default|SetOld_Rotator (Math|Rotator|Lerp(Rotator) (Class|KismetMathLibrary|MakeRot (* (Input|AxisValues|GetCam_Y) -1.0) (* (Input|AxisValues|GetCam_X) -1.0) 0.0) (Variables|Default|GetOld_Rotator) 0.9))
    (else
      (Transformation|AddRelativeRotation (Variables|Default|GetCamera_Mover) (Math|Rotator|Lerp(Rotator) "0, 0, 0" (Variables|Default|GetOld_Rotator) 0.96) false)
      (Variables|Default|SetOld_Rotator (Math|Rotator|Lerp(Rotator) "0, 0, 0" (Variables|Default|GetOld_Rotator) 0.96))))
  (Math|Float|CompareFloat _pitch -1e+01
    (:>
      (Transformation|SetRelativeRotation (Class|KismetMathLibrary|MakeRot -1e+01 _yaw _roll) false))
    (:==
      (Math|Float|CompareFloat _pitch -8e+01 :!label _label
        (:<
          (Transformation|SetRelativeRotation (Class|KismetMathLibrary|MakeRot -8e+01 _yaw _roll) false))))
    (:<
      (goto _label))))

(event Input|ActionEvents|InputActionCam_Move
  (:Pressed
    (Variables|Default|SetCam_Moving true))
  (:Released
    (Variables|Default|SetCam_Moving false)))

(fn ConstructionScript)