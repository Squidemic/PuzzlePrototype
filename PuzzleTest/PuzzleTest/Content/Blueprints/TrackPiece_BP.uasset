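; Rotatable track tile that turns 90 degrees in yaw when clicked and visually shows whether it connects to other pieces.
; The construction script applies the configured mesh and rotation, then adds trigger boxes for the sides enabled by the Top, Bottom, Right and Left flags.
; Each Tick scans those boxes for overlapping components tagged "Trigger" and switches the track and square meshes between active and inactive materials.
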(event Custom|Break%20Loop
  (Utilities|Array|ForEachLoopwithBreak (Variables|Default|GetTrigger%20Boxes)) ; enters at Break
)

(event EventActorOnClicked
  ;[1 1 1] Rotates piece when clicked
  (Variables|Default|SetRotation (+ (Variables|Default|GetRotation) 9e+01))
  (Transformation|SetActorRotation (Class|KismetMathLibrary|MakeRot 0.0 (Variables|Default|GetRotation) 0.0)))

(event EventTick
  (params (DeltaSeconds :type Float%20%28single-precision%29))
  (bind _array_element (Utilities|Array|ForEachLoopwithBreak (Variables|Default|GetTrigger%20Boxes))
    (:LoopBody
      (for _array_element_2 (Class|PrimitiveComponent|GetOverlappingComponents _array_element)
        (if (Components|ComponentHasTag _array_element_2 "Trigger")
          (Variables|Default|SetSet%20material true)
          (CallFunction|BreakLoop)
          (else
            (Variables|Default|SetSet%20material false)))))
    (:Completed
      (if (Variables|Default|GetSet%20material)
        ;[1 1 1] Events that happen when a connection is/is not made
        (Rendering|Material|SetMaterial (Variables|Default|GetTrack%20Piece%20Mesh) 0 "/Game/Meshes/MAT_Blocks.MAT_Blocks")
        (Rendering|Material|SetMaterial (Variables|Default|GetSquareMesh) 0 "/Game/Meshes/MAT_Square.MAT_Square")
        (else
          (Rendering|Material|SetMaterial (Variables|Default|GetTrack%20Piece%20Mesh) 0 "/Game/Meshes/MAT_Inactive2.MAT_Inactive2")
          (Rendering|Material|SetMaterial (Variables|Default|GetSquareMesh) 0 "/Game/Meshes/MAT_Inactive.MAT_Inactive"))))))

(fn ConstructionScript
  (Components|StaticMesh|SetStaticMesh (Variables|Default|GetTrack%20Piece))
  (Transformation|SetActorRotation (Class|KismetMathLibrary|MakeRot 0.0 (Variables|Default|GetRotation) 0.0))
  (Variables|Default|SetTrigger%20Booleans (Utilities|Array|MakeArray (Variables|Triggers|GetTop) (Variables|Triggers|GetBottom) (Variables|Triggers|GetRight) (Variables|Triggers|GetLeft)))
  (for (_array_element _array_index) (Variables|Default|GetTrigger%20Booleans)
    (if _array_element
      (bind _returnvalue (AddComponent|AddBoxComponent false (Utilities|Array|Get(acopy) (Variables|Default|GetTrigger%20Transformations) _array_index)))
      (Utilities|Array|Add (Variables|Default|GetTrigger%20Boxes) _returnvalue))))